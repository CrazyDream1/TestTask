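; BP_Turtle is the turtle actor Blueprint that supplies visual and audio feedback as the turtle starts, runs, stops and finishes.
; Four events drive paired effect and audio components: start and run activate their own pairs, while stop deactivates the run pair.
; Finish activates the finish pair and also shuts off the run pair.
; The graph holds no movement logic, and its BeginPlay, overlap and Tick events are unused.
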(event `EventOnStart`
  (`ActorComponent.Activate` (`self.StartEffect`) false)
  (`ActorComponent.Activate` (`self.AudioStart`) false))

(event `EventOnRun`
  (`ActorComponent.Activate` (`self.RunEffect`) false)
  (`ActorComponent.Activate` (`self.AudioRun`) false))

(event `EventOnStop`
  (`ActorComponent.Deactivate` (`self.RunEffect`))
  (`ActorComponent.Deactivate` (`self.AudioRun`)))

(event `EventOnFinish`
  (`ActorComponent.Activate` (`self.FinishEffect`) false)
  (`ActorComponent.Activate` (`self.AudioFinish`) false)
  (`ActorComponent.Deactivate` (`self.RunEffect`))
  (`ActorComponent.Deactivate` (`self.AudioRun`)))

(fn `UserConstructionScript`
  (`parent.UserConstructionScript`))