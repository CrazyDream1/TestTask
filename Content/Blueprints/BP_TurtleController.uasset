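; AI controller for BP_Turtle that sends the turtle to an End actor and signals each stage of its trip.
; StartMove caches the controlled pawn as a turtle, fires its start event, then calls Movement to trigger the move event.
; An AIMoveTo fires the turtle's run event once the move is issued and its finish event on success, with no failure handling.
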(event `EventMovementToEnd`
  (bind _controlledturtle (`self.ControlledTurtle`))
  (`|AIMoveTo` (`self.K2_GetPawn`) (0.0 0.0 0.0) (`self.End`) 1.0
    (:`then`
      (`/Game/Blueprints/BP_Turtle.EventOnRun` _controlledturtle))
    (:`OnSuccess`
      (`/Game/Blueprints/BP_Turtle.EventOnFinish` _controlledturtle))))

(fn `Movement`
  (`self.EventMovementToEnd`))

(fn `StartMove`
  (bind _output_get (set `self.ControlledTurtle` (cast `/Game/Blueprints/BP_Turtle` (`self.K2_GetPawn`) :!pure true)))
  (`/Game/Blueprints/BP_Turtle.EventOnStart` _output_get)
  (`self.Movement`))

(fn `UserConstructionScript`)