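; AI controller that drives a turtle toward an End actor, periodically backtracking toward Start.
; The movement event runs toward End for a set duration, then, if unfinished, retreats toward Start for another duration.
; It then calls Movement, which restarts the cycle and triggers the turtle's run event.
; Reaching End sets IsMovementDone, which halts the loop, and triggers the turtle's finish event.
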(event `EventMovementToEndWithBackwardMovement`
  (`|AIMoveTo` (`self.K2_GetPawn`) (0.0 0.0 0.0) (`self.End`) 1.0
    (:`then`
      (`KismetSystemLibrary.Delay` (`self.RunDuration`))
      (if (not (`self.IsMovementDone`))
        (`self.StopMovement`)
        (`|AIMoveTo` (`self.K2_GetPawn`) (0.0 0.0 0.0) (`self.Start`) 1.0
          (:`then`
            (`KismetSystemLibrary.Delay` (`self.BackwardDuration`))
            (`self.StopMovement`)
            (`self.Movement`)))))
    (:`OnSuccess`
      (set `self.IsMovementDone` true)
      (`/Game/Blueprints/BP_Turtle.EventOnFinish` (`self.ControlledTurtle`)))))

(fn `Movement`
  (if (not (`self.IsMovementDone`))
    (`self.EventMovementToEndWithBackwardMovement`)
    (`/Game/Blueprints/BP_Turtle.EventOnRun` (`self.ControlledTurtle`))))

(fn `UserConstructionScript`
  (`parent.UserConstructionScript`))