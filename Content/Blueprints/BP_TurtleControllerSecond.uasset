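; AI controller that drives a turtle pawn toward an End actor in alternating run and stop phases.
; A movement event starts AI MoveTo, halts it after RunDuration, waits StopDuration, then calls Movement to restart it unless finished.
; It fires run, stop and finish events on the controlled turtle, setting IsMovementDone when the move succeeds.
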(event `EventMovementToEndWithDelays`
  (`|AIMoveTo` (`self.K2_GetPawn`) (0.0 0.0 0.0) (`self.End`) 1.0
    (:`then`
      (`|ExecutionSequence`
        (:`then_0`
          (`/Game/Blueprints/BP_Turtle.EventOnRun` (`self.ControlledTurtle`)))
        (:`then_1`
          (`KismetSystemLibrary.Delay` (`self.RunDuration`))
          (`self.StopMovement`)
          (`|ExecutionSequence`
            (:`then_0`
              (`/Game/Blueprints/BP_Turtle.EventOnStop` (`self.ControlledTurtle`)))
            (:`then_1`
              (`KismetSystemLibrary.Delay` (`self.StopDuration`))
              (`self.Movement`))))))
    (:`OnSuccess`
      (set `self.IsMovementDone` true)
      (`/Game/Blueprints/BP_Turtle.EventOnFinish` (`self.ControlledTurtle`)))))

(fn `Movement`
  (if (not (`self.IsMovementDone`))
    (`self.EventMovementToEndWithDelays`)))

(fn `UserConstructionScript`
  (`parent.UserConstructionScript`))